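; Archer enemy Blueprint that turns to face the player each tick while it is alive and has detected them.
; Primary and secondary attacks both play the crossbow montage and share a short delayed arrow sound at the attack point.
; When the shot completes, an exhausted montage plays, and its completion sets the same cooldown flag for either attack.
; No projectile spawning or damage happens in this graph.
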(event EventBeginPlay
  (|CallParentFunction) ; This node is disabled and will not be called.\nDrag off pins to build functionality.
)

(event Collision|EventActorBeginOverlap
  (params (OtherActor :type Actor%20Object%20Reference))
  (|CallParentFunction OtherActor) ; This node is disabled and will not be called.\nDrag off pins to build functionality.
)

(event EventTick
  (params (DeltaSeconds :type Float%20%28single-precision%29))
  (|CallParentFunction DeltaSeconds)
  (if (and (Variables|Default|GetJugadorDetectado) (Variables|Default|GetEstoyVivo?))
    (CallFunction|RotarViendoAlJugador)))

(event EventAtaquePrimario
  (bind _mesh (Variables|Character|GetMesh))
  ;[1 0.07707 0] AtaquePrimario
  (Animation|Montage|PlayMontage _mesh "/Game/Assets/Animaciones/DisparoBallesta.DisparoBallesta"
    (:then
      (Utilities|FlowControl|Delay 0.3)
      (Audio|PlaySoundatLocation "/Game/Assets/sonidos/arrow.arrow" (Transformation|GetWorldLocation (Variables|Default|GetAtackPointEspada)) "0, 0, 0" 1.0 1.0 0.0 0 0 0 0))
    (:OnCompleted
      (Animation|Montage|PlayMontage _mesh "/Game/Assets/Animaciones/Agotado.Agotado"
        (:OnCompleted
          (Variables|Default|SetEnfriamiento1 true))))))

(event EventAtaqueSecundario
  (bind _mesh (Variables|Character|GetMesh))
  ;[1 0.07707 0] AtaqueSecundario
  (Animation|Montage|PlayMontage _mesh "/Game/Assets/Animaciones/DisparoBallesta.DisparoBallesta"
    (:then
      (Utilities|FlowControl|Delay 0.3)
      (Audio|PlaySoundatLocation "/Game/Assets/sonidos/arrow.arrow" (Transformation|GetWorldLocation (Variables|Default|GetAtackPointEspada)) "0, 0, 0" 1.0 1.0 0.0 0 0 0 0))
    (:OnCompleted
      (Animation|Montage|PlayMontage _mesh "/Game/Assets/Animaciones/Agotado.Agotado"
        (:OnCompleted
          (Variables|Default|SetEnfriamiento1 true))))))

(fn ConstructionScript
  (|CallParentFunction))