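; Enemy character that patrols waypoints, detects the player through PawnSensing, then chases and attacks until killed.
; Tick drives AI MoveTo and, in range, randomly picks one of two currently identical montage attacks, gated by a cooldown.
; Patrullar loops through waypoints with random pauses but is not started in this graph.
; On death it flags the animation Blueprint, increments the player's kill count, spawns a random drop and destroys itself.
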(event OnSeePawn(PawnSensing)
  (params (Pawn :type Pawn%20Object%20Reference))
  (Variables|Patrullar|SetJugadorDetectado true))

(event OnHearNoise(PawnSensing)
  (params (Instigator :type Pawn%20Object%20Reference) (Location :type Vector%20%28by%20ref%29 :default "0, 0, 0") (Volume :type Float%20%28single-precision%29))
  (Variables|Patrullar|SetJugadorDetectado true))

(event Custom|Patrullar
  ;[0 1 0.1305] Patrullar
  (if (Variables|Default|GetEstoyVivo?)
    (if (not (Variables|Patrullar|GetJugadorDetectado))
      (AI|AIMoveTo self "0, 0, 0" (Utilities|Array|Get(acopy) (Variables|Patrullar|GetrecorridoPatrulla) (Variables|Patrullar|GetpatrullaActual)) 5.0 false
        (:OnSuccess
          _)
        (:OnFail
          _))
      (Math|Integer|IncrementInt (Variables|Patrullar|GetpatrullaActual)
        (:%20%20
          (if (> (Variables|Patrullar|GetpatrullaActual) (Utilities|Array|Length (Variables|Patrullar|GetrecorridoPatrulla)))
            (Variables|Patrullar|SetpatrullaActual 0))
          (Utilities|FlowControl|Delay (Math|Random|RandomFloatinRange 0.0 2.0))
          (CallFunction|Patrullar))))))

(event EventBeginPlay
  (|CallParentFunction)
  (CallFunction|SetEnemigoBP)
  (if (Variables|Patrullar|GetJugadorDetectado)
    _))

(event Collision|EventActorBeginOverlap
  (params (OtherActor :type Actor%20Object%20Reference)))

(event EventTick
  (params (DeltaSeconds :type Float%20%28single-precision%29))
  (bind _returnvalue (Game|Player|GetPlayerPawn 0))
  (bind _drop (Variables|Default|GetDrop))
  (if (Variables|Default|GetEstoyVivo?)
    (if (Variables|Patrullar|GetJugadorDetectado)
      (if (Variables|Patrullar|GetAtacando)
        (Variables|Patrullar|SetAtacando false)
        (if (Variables|Default|GetEnfriamiento1)
          (Variables|Default|SetEnfriamiento1 false)
          (if (Math|Random|RandomBool)
            (CallFunction|AtaquePrimario)
            (else
              (CallFunction|AtaqueSecundario))))
        (elif (Variables|Default|GetEnfriamiento1)
          (AI|AIMoveTo self "0, 0, 0" _returnvalue (Variables|Patrullar|GetDistanciaAtaque) true
            (:OnSuccess
              (Variables|Patrullar|SetAtacando true))))))
    (elif (not (Variables|Default|GetMuerto))
      (Variables|Default|SetMuerto true)
      (Animation|StopAnimMontage (Animation|GetCurrentMontage :!class /Script/Engine.Character))
      (bind _asbp_animaciones (Utilities|Casting|CastToBP_Animaciones (Components|SkeletalMesh|GetAnimInstance (Variables|Character|GetMesh))))
      (Variables|/Game/Blueprints/Enemigos/BP_Animaciones.BP_Animaciones_C|SetMuerto _asbp_animaciones true)
      (bind _asbp_jugador (Utilities|Casting|CastToBP_Jugador _returnvalue))
      (Variables|/Game/Blueprints/Jugador/BP_Jugador.BP_Jugador_C|SetEnemigosMuertos _asbp_jugador (+ (Variables|/Game/Blueprints/Jugador/BP_Jugador.BP_Jugador_C|GetEnemigosMuertos _asbp_jugador) 1))
      (Utilities|FlowControl|Delay 2.0)
      ;[1 1 1] Drop item
      (Game|SpawnActorfromClass (Utilities|Array|Get(acopy) _drop (Math|Random|RandomIntegerinRange 0 (Utilities|Array|Length _drop))) (Math|Conversions|ToTransform(Vector) (.location (Transformation|GetWorldTransform (Variables|Default|Getcabeza)))) "Undefined" 0 0)
      (Actor|DestroyActor))))

(event EventAtaquePrimario
  (bind _mesh (Variables|Character|GetMesh))
  ;[1 0.07707 0] AtaquePrimario
  (Animation|Montage|PlayMontage _mesh "/Game/Assets/Animaciones/AtacandoEnemigo.AtacandoEnemigo"
    (:OnCompleted
      (Animation|Montage|PlayMontage _mesh "/Game/Assets/Animaciones/Agotado.Agotado"
        (:OnCompleted
          (Variables|Default|SetEnfriamiento1 true))))))

(event EventAtaqueSecundario
  (bind _mesh (Variables|Character|GetMesh))
  ;[1 0.07707 0] AtaqueSecundario
  (Animation|Montage|PlayMontage _mesh "/Game/Assets/Animaciones/AtacandoEnemigo.AtacandoEnemigo"
    (:OnCompleted
      (Animation|Montage|PlayMontage _mesh "/Game/Assets/Animaciones/Agotado.Agotado"
        (:OnCompleted
          (Variables|Default|SetEnfriamiento1 true))))))

(fn ConstructionScript
  (|CallParentFunction))

(fn SetEnemigoBP
  (bind _asbp_animaciones (Utilities|Casting|CastToBP_Animaciones (Components|SkeletalMesh|GetAnimInstance (Variables|Character|GetMesh))))
  (Variables|/Game/Blueprints/Enemigos/BP_Animaciones.BP_Animaciones_C|SetEnemigos _asbp_animaciones self))