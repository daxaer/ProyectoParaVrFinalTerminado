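; Door actor that swings open when the player overlaps it after killing enough enemies to meet its target count.
; The overlap compares BP_Jugador's EnemigosMuertos against ObjetivoParaAbrir, then plays a sound and a timeline that rotates the door's yaw.
; PrimeraVez limits opening to a single time.
; A separate Cerrar event, not called within this graph, reverses the timeline with the same sound when CerrarPuerta is set.
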(event Custom|Cerrar
  (if (Variables|Default|GetCerrarPuerta)
    (CallFunction|ReproducirSonido)
    (Variables|Default|SetprimeraVez false)
    (bind _rotarpuerta (Timeline|Abrir Reverse)
      (:Update
        (Transformation|SetRelativeRotation (Variables|Default|GetPuerta) (Math|Rotator|MakeRotator 0.0 0.0 _rotarpuerta) false false)))))

(event Custom|AbrirPuerta
  (if (Variables|Default|GetprimeraVez)
    (CallFunction|ReproducirSonido)
    (Variables|Default|SetprimeraVez false)
    (bind _rotarpuerta (Timeline|Abrir Play)
      (:Update
        (Transformation|SetRelativeRotation (Variables|Default|GetPuerta) (Math|Rotator|MakeRotator 0.0 0.0 _rotarpuerta) false false)))))

(event Custom|ReproducirSonido
  (Audio|PlaySoundatLocation (Variables|Default|GetSound) (Transformation|GetWorldLocation (Variables|Default|GetPuerta)) "0, 0, 0" 1.0 1.0 0.0 0 0 0 0))

(event Collision|EventActorBeginOverlap
  (params (OtherActor :type Actor%20Object%20Reference))
  (bind _returnvalue (Game|Player|GetPlayerPawn 0))
  (if (== OtherActor _returnvalue)
    (bind _asbp_jugador (Utilities|Casting|CastToBP_Jugador _returnvalue))
    (if (>= (Variables|/Game/Blueprints/Jugador/BP_Jugador.BP_Jugador_C|GetEnemigosMuertos _asbp_jugador) (Variables|Default|GetObjetivo%20Para%20Abrir))
      (CallFunction|AbrirPuerta))))

(fn ConstructionScript)