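; PickUps is a health potion pickup that heals the player pawn (BP_Jugador) on overlap.
; If Vida is below MaxVida, it plays a heal sound, adds RestaurarVida, caps the result at MaxVida and destroys itself.
; The Heal.UpdateHeal call runs only when the value gets capped.
; At full health it plays an error sound and stays in the world.
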(event Collision|EventActorBeginOverlap
  (params (OtherActor :type Actor%20Object%20Reference))
  (bind _returnvalue (Game|Player|GetPlayerPawn 0))
  (if (== OtherActor _returnvalue)
    (bind _asbp_jugador (Utilities|Casting|CastToBP_Jugador _returnvalue))
    (if (> (Variables|/Game/Blueprints/BP_Personajes.BP_Personajes_C|GetMaxVida _asbp_jugador) (Variables|/Game/Blueprints/BP_Personajes.BP_Personajes_C|GetVida _asbp_jugador))
      (Audio|PlaySound2D "/Game/Assets/sonidos/healUp.healUp" 1.0 1.0 0.0 0 0)
      (bind _output_get (Variables|/Game/Blueprints/BP_Personajes.BP_Personajes_C|SetVida _asbp_jugador (+ (Variables|/Game/Blueprints/BP_Personajes.BP_Personajes_C|GetVida _asbp_jugador) (Variables|Default|GetRestaurarVida))))
      (if (> _output_get (Variables|/Game/Blueprints/BP_Personajes.BP_Personajes_C|GetMaxVida _asbp_jugador))
        (bind _output_get_2 (Variables|/Game/Blueprints/BP_Personajes.BP_Personajes_C|SetVida _asbp_jugador (Variables|/Game/Blueprints/BP_Personajes.BP_Personajes_C|GetMaxVida _asbp_jugador)))
        (Default|UpdateHeal (Variables|/Game/Blueprints/BP_Personajes.BP_Personajes_C|GetHeal _asbp_jugador) _output_get_2))
      (Actor|DestroyActor)
      (else
        (Audio|PlaySound2D "/Game/Assets/sonidos/error.error" 1.0 1.0 0.0 0 0)))))

(fn ConstructionScript)