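; BP_Personajes is a base character Blueprint providing shared health, damage, cooldown and facing logic, with empty primary and secondary attack events.
; Health starts at maximum; AnyDamage subtracts it with clamping, playing hurt or death sounds and clearing EstoyVivo at zero.
; A player-specific damage function also updates the Heal display.
; Two delay-based events reset cooldowns, and a helper smoothly yaws enemies toward BP_Jugador using RInterpTo.
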(event Custom|RotarViendoAlJugador
  (bind _asbp_jugador (Utilities|Casting|CastToBP_Jugador (Game|Player|GetPlayerPawn 0)))
  (bind _rotacionaljugador (CallFunction|MirarAlJugador self _asbp_jugador))
  (Transformation|SetActorRotation _rotacionaljugador))

(event Custom|ResetEnfriamiento2
  (Variables|Enfriamientos|SetEnfriamiento2 false)
  (Utilities|FlowControl|Delay (Variables|Enfriamientos|GetEnfriamientoActual2))
  (Variables|Enfriamientos|SetEnfriamiento2 true))

(event Custom|ResetEnfriamiento1
  (Variables|Enfriamientos|SetEnfriamiento1 false)
  (Utilities|FlowControl|Delay (Variables|Enfriamientos|GetEnfriamientoActual1))
  (Variables|Enfriamientos|SetEnfriamiento1 true))

(event Custom|ReproducirSonidoDaño
  ;[1 0 0] SonidoRecibirDaño
  (Audio|PlaySound2D (Variables|Default|GetDañado) 1.0 1.0 0.0 0 0))

(event Custom|AtaqueSecundario)

(event Custom|AtaquePrimario)

(event EventBeginPlay
  (CallFunction|VidaInicial))

(event Game|Damage|EventAnyDamage
  (params (Damage :type Float%20%28single-precision%29) (DamageType :type Damage%20Type%20Object%20Reference) (InstigatedBy :type Controller%20Object%20Reference) (DamageCauser :type Actor%20Object%20Reference))
  (CallFunction|RestarVida Damage))

(fn ConstructionScript)

(fn VidaInicial
  (Variables|VIda|SetVida (Variables|Vida|GetMaxVida)))

(fn RestarVida
  (params (B :type Float%20%28double-precision%29))
  (if (not (and (Variables|VIda|GetInvulnerabilidad) (not (Variables|VIda|GetEstoyVivo?))))
    (bind _output_get (Variables|VIda|SetVida (Math|Float|Clamp(Float) (- (Variables|VIda|GetVida) B) 0.0 (Variables|Vida|GetMaxVida))))
    (if (== _output_get 0.0)
      (Variables|VIda|SetEstoyVivo? false)
      (Audio|PlaySound2D (Variables|Default|GetDead) 1.0 1.0 0.0 0 0)
      (else
        (CallFunction|ReproducirSonidoDaño)))))

(fn MirarAlJugador
  (params (Enemigo :type Actor%20Object%20Reference) (Player :type Actor%20Object%20Reference))
  (return (Math|Interpolation|RInterpTo (Transformation|GetActorRotation Enemigo) (Math|Rotator|MakeRotator 0.0 0.0 (.Yaw (Math|Rotator|BreakRotator (Math|Rotator|FindLookatRotation (Transformation|GetActorLocation Enemigo) (Transformation|GetActorLocation Player))))) (Utilities|Time|GetWorldDeltaSeconds) 5.0)))

(fn RestarVidaPlayer
  (params (daño :type Float%20%28double-precision%29))
  (if (not (and (Variables|VIda|GetInvulnerabilidad) (not (Variables|VIda|GetEstoyVivo?))))
    (bind _output_get (Variables|VIda|SetVida (Math|Float|Clamp(Float) (- (Variables|VIda|GetVida) daño) 0.0 (Variables|Vida|GetMaxVida))))
    (Default|UpdateHeal (Variables|Default|GetHeal) _output_get)
    (if (== _output_get 0.0)
      (Variables|VIda|SetEstoyVivo? false)
      (Audio|PlaySound2D (Variables|Default|GetDead) 1.0 1.0 0.0 0 0)
      (else
        (CallFunction|ReproducirSonidoDaño)))))